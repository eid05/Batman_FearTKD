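; Thug enemy that chases the player on sight and can be killed by Fear Takedowns.
; Proximity starts timers driving custom-depth outline, player-facing icon and random scared montages while the player is in FTD.
; PawnSensing and Tick drive AIMoveTo chase and last-seen search; the random wander loop is disconnected.
; Kill picks a takedown animation from the player's fear direction and index, then ragdolls with an impulse, optionally destroying the body.
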(event `self.PlayerDetector.OnComponentBeginOverlap`
  (params (OverlappedComponent :type "PrimitiveComponent Object Reference") (OtherActor :type "Actor Object Reference") (OtherComp :type "PrimitiveComponent Object Reference") (OtherBodyIndex :type Integer) (bFromSweep :type Boolean) (SweepResult :type "HitResult Structure (by ref)"))
  ;[0.3125 0.3125 0.3125] Overlap
  (if (not (`self.IsDead?`))
    (`KismetSystemLibrary.K2_SetTimer` null "SetCrosshair" 0.01 true)
    (`KismetSystemLibrary.K2_SetTimer` null "FearOutline" 0.01 true)
    (`SceneComponent.SetVisibility` (`self.Widget`) true true)
    (set `PrimitiveComponent.bGenerateOverlapEvents` true (`self.BackCone`))))

(event `FearOutline`
  (bind _mesh (`self.Mesh`))
  (bind _returnvalue (`SceneComponent.K2_GetComponentLocation` (`self.Mesh`)))
  ;[1 1 1] Outline
  (bind (_outhit _returnvalue_2) (`KismetSystemLibrary.SphereTraceSingleForObjects` _returnvalue (+ _returnvalue 1.0) 1064.0 (`|MakeArray` "ObjectTypeQuery9" :!type "EObjectTypeQuery Enum")))
  (if _returnvalue_2
    (if (not (`self.IsDead?`))
      (`PrimitiveComponent.SetRenderCustomDepth` _mesh true)
      (set `self.Overlapped?` true)
      (else
        (`PrimitiveComponent.SetRenderCustomDepth` _mesh false :!label _label)
        (set `self.Overlapped?` false)))
    (else
      (goto _label))))

(event `self.PlayerDetector.OnComponentEndOverlap`
  (params (OverlappedComponent :type "PrimitiveComponent Object Reference") (OtherActor :type "Actor Object Reference") (OtherComp :type "PrimitiveComponent Object Reference") (OtherBodyIndex :type Integer))
  ;[0.3125 0.3125 0.3125] Overlap
  (`KismetSystemLibrary.K2_ClearTimer` null "FearOutline")
  (`PrimitiveComponent.SetRenderCustomDepth` (`self.Mesh`) false)
  (set `self.Icon` false)
  (set `self.Overlapped?` false)
  (`SceneComponent.SetVisibility` (`self.Widget`) false true)
  (`KismetSystemLibrary.Delay` 0.1)
  (`KismetSystemLibrary.K2_ClearTimer` null "SetCrosshair")
  (set `PrimitiveComponent.bGenerateOverlapEvents` false (`self.BackCone`)))

(event `SetCrosshair`
  (bind _widget (`self.Widget`))
  (bind _widget_2 (`self.Widget`))
  (bind _returnvalue (`SceneComponent.K2_GetComponentScale` (`self.Widget`)))
  ;[1 1 1] SetCrosshair
  (`|ExecutionSequence`
    (:`then_0`
      (bind _outhit (`KismetSystemLibrary.LineTraceSingle` (`self.K2_GetActorLocation`) (`self.K2_GetActorLocation` (`GameplayStatics.GetPlayerPawn` 0)) "TraceTypeQuery1"))
      (`SceneComponent.K2_SetWorldRotation` _widget_2 (`KismetMathLibrary.MakeRotator` 0.0 (`KismetMathLibrary.ClampAngle` (.pitch (`KismetMathLibrary.FindLookAtRotation` (`SceneComponent.K2_GetComponentLocation` _widget_2) (`.TraceEnd` (`GameplayStatics.BreakHitResult` _outhit)))) 0.0 90.0) (.yaw (`KismetMathLibrary.FindLookAtRotation` (`SceneComponent.K2_GetComponentLocation` _widget_2) (`.TraceEnd` (`GameplayStatics.BreakHitResult` _outhit))))) false false))
    (:`then_1`
      (if (`self.Icon`)
        (bind (_direction _lerp) (`Timeline|IconTrueTL`)
          (:`Update`
            (`SceneComponent.SetWorldScale3D` _widget (`KismetMathLibrary.VLerp` _returnvalue (0.04 0.04 0.04) _lerp)))
          (:`Finished`
            (`TimelineComponent.SetNewTime` (`self.IconTrueTL`) 0.0)))
        (else
          (bind (_direction_2 _lerp_2) (`Timeline|IconFalseTL`)
            (:`Update`
              (`SceneComponent.SetWorldScale3D` _widget (`KismetMathLibrary.VLerp` _returnvalue (0.0 0.0 0.0) _lerp_2)))
            (:`Finished`
              (`TimelineComponent.SetNewTime` (`self.IconFalseTL`) 0.0))))))
    (:`then_2`
      (if (`/Game/DefaultAssets/Blueprints/Player/ThirdPersonCharacter.IsInFTD` (cast `/Game/DefaultAssets/Blueprints/Player/ThirdPersonCharacter` (`GameplayStatics.GetPlayerPawn` 0) :!pure true))
        (`/Engine/EditorBlueprintResources/StandardMacros.DoOnce` false :!label _label_2
          (:`Completed`
            (`|PlayMontage` (`self.Mesh`) (select `int` (`KismetMathLibrary.RandomIntegerInRange` 0 4) :`0` "/Game/DefaultAssets/CharacterAssets/Mannequin/Animations/Enemy/Fear/Scared/SCR_Beg_For_Life_Standing_Loop_Montage.SCR_Beg_For_Life_Standing_Loop_Montage" :`1` "/Game/DefaultAssets/CharacterAssets/Mannequin/Animations/Enemy/Fear/Scared/SCR_Gunpoint_Hands_Up_Start_Montage.SCR_Gunpoint_Hands_Up_Start_Montage" :`2` "/Game/DefaultAssets/CharacterAssets/Mannequin/Animations/Enemy/Fear/Scared/SCR_Stand_Scared_Front_To_Back_Up_Montage.SCR_Stand_Scared_Front_To_Back_Up_Montage" :`3` "/Game/DefaultAssets/CharacterAssets/Mannequin/Animations/Enemy/Fear/Scared/SCR_Stand_Scared_Front_To_Creeping_Back_Montage.SCR_Stand_Scared_Front_To_Creeping_Back_Montage" :`4` "/Game/DefaultAssets/CharacterAssets/Mannequin/Animations/Enemy/Fear/Scared/SCR_Stand_Spooked_Fall_Down_Stand_Montage.SCR_Stand_Spooked_Fall_Down_Stand_Montage" :!type "AnimMontage Object Reference") 0.8
              (:`OnCompleted`
                (goto _label_2 :!via `Reset`))
              (:`OnBlendOut`
                (goto _label_2 :!via `Reset`)))))))))

(event `Kill`
  (bind (_returnvalue_roll _returnvalue_pitch _returnvalue_yaw) (`KismetMathLibrary.BreakRotator` (`self.K2_GetActorRotation`)))
  (bind _mesh (`self.Mesh`))
  (bind _mesh_2 (`self.Mesh`))
  (bind _mesh_3 (`self.Mesh`))
  (bind _mesh_4 (`self.Mesh`))
  (bind _mesh_5 (`self.Mesh`))
  (bind _mesh_6 (`self.Mesh`))
  (bind (_returnvalue_x _returnvalue_y _returnvalue_z) (`KismetMathLibrary.BreakVector` (`SceneComponent.GetForwardVector` _mesh_5)))
  (bind _asthird_person_character (cast `/Game/DefaultAssets/Blueprints/Player/ThirdPersonCharacter` (`GameplayStatics.GetPlayerPawn` 0) :!pure true))
  ;[1 1 1] Kill Event
  (set `self.Icon` false)
  (set `self.Overlapped?` false)
  (set `self.IsDead?` true)
  (`KismetSystemLibrary.K2_ClearTimer` null "SetCrosshair")
  (`KismetSystemLibrary.K2_ClearTimer` null "FearOutline")
  (`PrimitiveComponent.SetRenderCustomDepth` (`self.Mesh`) false)
  (`TimelineComponent.Play` (`self.IconFalseTL`))
  (`|ExecutionSequence`
    (:`then_0`
      (`KismetSystemLibrary.Delay` 0.1)
      (`SceneComponent.SetVisibility` (`self.Widget`) false true))
    (:`then_1`
      (if (`self.HideDeadBody?`)
        (`KismetSystemLibrary.Delay` 5.0)
        (`self.K2_DestroyActor`)
        (else
          (`self.SetActorTickEnabled` false))))
    (:`then_2`
      (`PrimitiveComponent.SetCollisionEnabled` (`self.CapsuleComponent`) "NoCollision")
      (if (`/Game/DefaultAssets/Blueprints/Player/ThirdPersonCharacter.FearFront` _asthird_person_character)
        (switch `/Game/DefaultAssets/Blueprints/Player/FearDirection` (`/Game/DefaultAssets/Blueprints/Player/ThirdPersonCharacter.FearDirection` _asthird_person_character)
          (:`NewEnumerator0`
            ;[1 1 1] Front
            (`SceneComponent.K2_SetWorldRotation` _mesh_6 (`KismetMathLibrary.MakeRotator` _returnvalue_roll _returnvalue_pitch (+ _returnvalue_yaw 90.0)) false false)
            (switch `int` (`/Game/DefaultAssets/Blueprints/Player/ThirdPersonCharacter.FearIndex` _asthird_person_character)
              (:`0`
                (`SkeletalMeshComponent.PlayAnimation` _mesh_6 "/Game/DefaultAssets/CharacterAssets/Mannequin/Animations/Enemy/Fear/Front/Thug_Fear_Takedown_Front_0-2.Thug_Fear_Takedown_Front_0-2" false)
                (`KismetSystemLibrary.Delay` 2.26))
              (:`1`
                (`SkeletalMeshComponent.PlayAnimation` _mesh_6 "/Game/DefaultAssets/CharacterAssets/Mannequin/Animations/Enemy/Fear/Front/Thug_Fear_Takedown_Front_1.Thug_Fear_Takedown_Front_1" false)
                (`KismetSystemLibrary.Delay` 1.92))
              (:`2`
                (`SkeletalMeshComponent.PlayAnimation` _mesh_6 "/Game/DefaultAssets/CharacterAssets/Mannequin/Animations/Enemy/Fear/Front/Thug_Fear_Takedown_Front_3.Thug_Fear_Takedown_Front_3" false)
                (`KismetSystemLibrary.Delay` 2.4))
              (:`3`
                (`SkeletalMeshComponent.PlayAnimation` _mesh_6 "/Game/DefaultAssets/CharacterAssets/Mannequin/Animations/Enemy/Fear/Front/Thug_Fear_Takedown_Front_4.Thug_Fear_Takedown_Front_4" false)
                (`KismetSystemLibrary.Delay` 2.44))))
          (:`NewEnumerator1`
            ;[1 1 1] Back
            (switch `int` (`/Game/DefaultAssets/Blueprints/Player/ThirdPersonCharacter.FearIndex` _asthird_person_character)
              (:`0`
                (`SkeletalMeshComponent.PlayAnimation` _mesh_3 "/Game/DefaultAssets/CharacterAssets/Mannequin/Animations/Enemy/Fear/Back/Thug_Fear_Takedown_Back_0-2.Thug_Fear_Takedown_Back_0-2" false)
                (`KismetSystemLibrary.Delay` 2.0))
              (:`1`
                (`SkeletalMeshComponent.PlayAnimation` _mesh_3 "/Game/DefaultAssets/CharacterAssets/Mannequin/Animations/Enemy/Fear/Back/Thug_Fear_Takedown_Back_1.Thug_Fear_Takedown_Back_1" false)
                (`KismetSystemLibrary.Delay` 1.56))
              (:`2`
                (`SceneComponent.SetWorldScale3D` _mesh_3 (-1.0 1.0 1.0))
                (`SkeletalMeshComponent.PlayAnimation` _mesh_3 "/Game/DefaultAssets/CharacterAssets/Mannequin/Animations/Enemy/Fear/Back/Thug_Fear_Takedown_Back_3.Thug_Fear_Takedown_Back_3" false)
                (`KismetSystemLibrary.Delay` 1.813708)
                (`SceneComponent.SetWorldScale3D` _mesh_3 (1.0 1.0 1.0))
                (`KismetSystemLibrary.Delay` 0.01))
              (:`3`
                (`SkeletalMeshComponent.PlayAnimation` _mesh_3 "/Game/DefaultAssets/CharacterAssets/Mannequin/Animations/Enemy/Fear/Back/Thug_Fear_Takedown_Back_4_Montage.Thug_Fear_Takedown_Back_4_Montage" false)
                (`KismetSystemLibrary.Delay` 1.9))))
          (:`NewEnumerator2`
            ;[1 1 1] Left
            (switch `int` (`/Game/DefaultAssets/Blueprints/Player/ThirdPersonCharacter.FearIndex` _asthird_person_character)
              (:`0`
                (`SkeletalMeshComponent.PlayAnimation` _mesh_4 "/Game/DefaultAssets/CharacterAssets/Mannequin/Animations/Enemy/Fear/Left/Thug_Fear_Takedown_Left_0-2.Thug_Fear_Takedown_Left_0-2" false)
                (`KismetSystemLibrary.Delay` 1.47))
              (:`1`
                (`SkeletalMeshComponent.PlayAnimation` _mesh_4 "/Game/DefaultAssets/CharacterAssets/Mannequin/Animations/Enemy/Fear/Left/Thug_Fear_Takedown_Left_1.Thug_Fear_Takedown_Left_1" false)
                (`KismetSystemLibrary.Delay` 1.47))
              (:`2`
                (`SkeletalMeshComponent.PlayAnimation` _mesh_4 "/Game/DefaultAssets/CharacterAssets/Mannequin/Animations/Enemy/Fear/Left/Thug_Fear_Takedown_Left_3.Thug_Fear_Takedown_Left_3" false)
                (`KismetSystemLibrary.Delay` 2.31))
              (:`3`
                (`SkeletalMeshComponent.PlayAnimation` _mesh_4 "/Game/DefaultAssets/CharacterAssets/Mannequin/Animations/Enemy/Fear/Left/Thug_Fear_Takedown_Left_4.Thug_Fear_Takedown_Left_4" false)
                (`KismetSystemLibrary.Delay` 1.64))))
          (:`NewEnumerator3`
            ;[1 1 1] Right
            (switch `int` (`/Game/DefaultAssets/Blueprints/Player/ThirdPersonCharacter.FearIndex` _asthird_person_character)
              (:`0`
                (`SkeletalMeshComponent.PlayAnimation` _mesh "/Game/DefaultAssets/CharacterAssets/Mannequin/Animations/Enemy/Fear/Right/Thug_Fear_Takedown_Right_0-2.Thug_Fear_Takedown_Right_0-2" false)
                (`KismetSystemLibrary.Delay` 1.55))
              (:`1`
                (`SkeletalMeshComponent.PlayAnimation` _mesh "/Game/DefaultAssets/CharacterAssets/Mannequin/Animations/Enemy/Fear/Right/Thug_Fear_Takedown_Right_1.Thug_Fear_Takedown_Right_1" false)
                (`KismetSystemLibrary.Delay` 1.43))
              (:`2`
                (`SkeletalMeshComponent.PlayAnimation` _mesh "/Game/DefaultAssets/CharacterAssets/Mannequin/Animations/Enemy/Fear/Right/Thug_Fear_Takedown_Right_3-4.Thug_Fear_Takedown_Right_3-4" false :!label _label_3)
                (`KismetSystemLibrary.Delay` 1.6))
              (:`3`
                (goto _label_3)))))
        (else
          ;[1 1 1] Back2
          (switch `int` (`/Game/DefaultAssets/Blueprints/Player/ThirdPersonCharacter.FearIndex` _asthird_person_character)
            (:`0`
              (`SkeletalMeshComponent.PlayAnimation` _mesh_2 "/Game/DefaultAssets/CharacterAssets/Mannequin/Animations/Enemy/Fear/Back/Thug_Fear_Takedown_Back2_0-2-4.Thug_Fear_Takedown_Back2_0-2-4" false :!label _label_4))
            (:`1`
              (`SkeletalMeshComponent.PlayAnimation` _mesh_2 "/Game/DefaultAssets/CharacterAssets/Mannequin/Animations/Enemy/Fear/Back/Thug_Fear_Takedown_Back2_1-3.Thug_Fear_Takedown_Back2_1-3" false :!label _label_5))
            (:`2`
              (goto _label_4))
            (:`3`
              (goto _label_5)))
          (`KismetSystemLibrary.Delay` 2.313708)))
      (`PrimitiveComponent.SetCollisionEnabled` _mesh_5 "PhysicsOnly")
      (`PrimitiveComponent.SetSimulatePhysics` _mesh_5 true)
      (`KismetSystemLibrary.Delay` 0.1)
      (if (`SceneComponent.IsSimulatingPhysics` _mesh_5 "root")
        (`PrimitiveComponent.AddImpulse` _mesh_5 (`KismetMathLibrary.MakeVector` (* _returnvalue_x 100000.0) (* _returnvalue_y 100000.0) _returnvalue_z) "None" false)))))

(event `self.ReceiveBeginPlay`
  ;[1 1 1] On see pawn
  (bind _output_get (set `self.Random Location` (`NavigationSystemV1.K2_GetRandomLocationInNavigableRadius` (`self.K2_GetActorLocation`) 1000.0 null null)))
  (`KismetSystemLibrary.PrintString` (`KismetStringLibrary.Conv_VectorToString` _output_get) false)
  (`self.Random Location Move`))

(event `self.BackCone.OnComponentBeginOverlap`
  (params (OverlappedComponent :type "PrimitiveComponent Object Reference") (OtherActor :type "Actor Object Reference") (OtherComp :type "PrimitiveComponent Object Reference") (OtherBodyIndex :type Integer) (bFromSweep :type Boolean) (SweepResult :type "HitResult Structure (by ref)"))
  (set `self.Back?` true))

(event `Random Location Move`
  ;[1 1 1] On see pawn
)

(event `self.BackCone.OnComponentEndOverlap`
  (params (OverlappedComponent :type "PrimitiveComponent Object Reference") (OtherActor :type "Actor Object Reference") (OtherComp :type "PrimitiveComponent Object Reference") (OtherBodyIndex :type Integer))
  (set `self.Back?` false))

(event `self.PawnSensing.OnSeePawn`
  (params (Pawn :type "Pawn Object Reference"))
  ;[1 1 1] On see pawn
  (set `self.SawPlayer` true)
  (`|ExecutionSequence`
    (:`then_0`
      (`KismetSystemLibrary.PrintString` "I see you" false))
    (:`then_1`
      (`KismetSystemLibrary.RetriggerableDelay` 0.5)
      (set `self.SawPlayer` false)
      (`|AIMoveTo` self (`self.last actor location`) null
        (:`OnSuccess`
          (`KismetSystemLibrary.PrintString` "onlastplace" false)
          (`|AIMoveTo` self (`self.last actor location + look`) null
            (:`OnSuccess`
              (`KismetSystemLibrary.PrintString` "Looking at last place" false)
              (`self.Random Location Move`))))))))

(event `self.ReceiveTick`
  (params (DeltaSeconds :type "Float (single-precision)"))
  (bind _returnvalue (`GameplayStatics.GetPlayerPawn` 0))
  (bind _returnvalue_2 (`self.K2_GetActorLocation` _returnvalue))
  ;[1 1 1] On see pawn
  (if (`self.SawPlayer`)
    (bind _asthird_person_character (cast `/Game/DefaultAssets/Blueprints/Player/ThirdPersonCharacter` _returnvalue))
    (`|AIMoveTo` self _returnvalue_2 _asthird_person_character
      (:`OnFail`
        (bind _output_get (set `self.last actor location` _returnvalue_2))
        (`KismetSystemLibrary.PrintString` (`KismetStringLibrary.Conv_VectorToString` _output_get) false)
        (`KismetSystemLibrary.Delay` 4.0)
        (bind _output_get_2 (set `self.last actor location + look` _returnvalue_2))
        (`KismetSystemLibrary.PrintString` (`KismetStringLibrary.Conv_VectorToString` _output_get_2) false)))))

(fn `UserConstructionScript`)